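; GM_LMA is the game mode that runs a countdown match timer.
; BeginPlay starts a looping one-second timer, whose custom event decrements GameTime.
; When the count reaches zero, it clears the timer, adds the WBP_MenuDeath widget to the viewport and shows the mouse cursor.
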(event `self.ReceiveBeginPlay`
  (bind _returnvalue (`KismetSystemLibrary.K2_SetTimerDelegate` (delegate `CustomEvent`) 1.0 true))
  (set `self.GameTimerHandle` _returnvalue))

(event `CustomEvent`
  (bind _output_get (set `self.GameTime` (- (`self.GameTime`) 1)))
  (if (== _output_get 0)
    (`KismetSystemLibrary.K2_ClearAndInvalidateTimerHandle` (`self.GameTimerHandle`))
    (bind _returnvalue (`|CreateWidget` "/Game/LeaveMeAlone/Widgets/UI/WBP_MenuDeath.WBP_MenuDeath_C"))
    (`UserWidget.AddToViewport` _returnvalue 0)
    (set `PlayerController.bShowMouseCursor` true (`GameplayStatics.GetPlayerController` 0))))

(fn `UserConstructionScript`)